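; Drivable vehicle Blueprint that switches the player's view to a CameraActor_Blueprint on BeginPlay and drives through physics.
; Forward input applies impulses along the forward vector below a speed cap.
; Right input applies an offset force and also sets yaw directly, zeroing pitch and roll, despite that step's OLD label.
; Both inputs act only when a short downward line trace reports ground nearby.
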(event EventBeginPlay
  (bind _outactors (Actor|GetAllActorsOfClass "/Game/CameraActor_Blueprint.CameraActor_Blueprint_C"))
  (Game|Player|SetViewTargetwithBlend (Game|GetPlayerController 0) (Utilities|Array|Get(acopy) _outactors) 0.0 "VTBlend_Linear" 0.0 false))

(event Input|AxisEvents|InputAxisForward
  (params (AxisValue :type Float%20%28single-precision%29))
  (bind _nearground (CallFunction|IsonGround))
  (if (and (< (Math|Vector|VectorLength (Transformation|GetVelocity)) 3e+03) _nearground)
    ;[1 1 1] car acceleration
    (Physics|AddImpulse (* (Math|Vector|GetForwardVector) (* (* AxisValue -1.0) 2.5e+05)) "None" false)))

(event Input|AxisEvents|InputAxisRight
  (params (AxisValue :type Float%20%28single-precision%29))
  (bind _returnvalue (Transformation|GetActorRightVector))
  (bind _nearground (CallFunction|IsonGround))
  (if _nearground
    ;[1 1 1] car rotation
    (Class|PrimitiveComponent|AddForceatLocation (* (* _returnvalue AxisValue) -1.7e+06) (+ (* _returnvalue -2e+02) (Transformation|GetActorLocation) (* (Transformation|GetActorForwardVector) -2e+02)) "None")
    ;[1 1 1] (OLD) instant yaw rotation
    (Transformation|SetActorRotation (Class|KismetMathLibrary|MakeRot 0.0 (+ (.Yaw (Class|KismetMathLibrary|BreakRot (Transformation|GetActorRotation))) (* AxisValue 2.0)) 0.0))))

(fn ConstructionScript)

(fn IsonGround
  (bind _returnvalue (Transformation|GetActorLocation))
  (bind _outhit (Collision|LineTraceByChannel _returnvalue (+ _returnvalue "0, 0,-200.000000") "TraceTypeQuery1" false 0 "None"))
  (return (< (Math|Vector|VectorLength (- (Transformation|GetActorLocation) (.Location (Collision|BreakHitResult _outhit)))) 8e+01)))