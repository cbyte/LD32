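; BotCar is an AI traffic car that drives at a random top speed and changes lanes around other vehicles.
; Each tick, a Drive/Left/Right state machine uses traces and box overlaps to overtake left, match a slower blocker's speed, or move right when clear.
; Physics impulses propel it while grounded below target speed.
; Lane changes reverse steering at the midpoint, combining an offset force with direct yaw rotation.
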(event EventTick
  (params (DeltaSeconds :type Float%20%28single-precision%29))
  (bind _returnvalue (Transformation|GetActorLocation))
  (bind _returnvalue_2 (Transformation|GetActorLocation))
  (bind _returnvalue_3 (Transformation|GetActorLocation))
  (bind _returnvalue_4 (Components|GetOwner))
  (bind _y (Math|Vector|BreakVector _returnvalue_2))
  (bind _returnvalue_5 (Transformation|GetActorLocation _returnvalue_4))
  (bind _y_2 (Math|Vector|BreakVector _returnvalue_3))
  (bind _y_3 (Math|Vector|BreakVector _returnvalue_5))
  ;[1 1 1] speed limit
  (bind _nearground (CallFunction|IsonGround))
  (if (and _nearground (< (Math|Vector|VectorLength (Transformation|GetVelocity)) (Variables|Default|Getspeed)))
    ;[1 1 1] car acceleration
    (Physics|AddImpulse (* (Math|Vector|GetForwardVector) (* (* (Variables|Default|Getspeed) -1.0) 2.5e+02)) "None" false))
  (switch Utilities|FlowControl|Switch|SwitchonDriveEnum (Variables|Default|Getstate)
    (:NewEnumerator0
      ;[1 1 1] Drive Forward
      (bind (_outhit _returnvalue_6) (Collision|LineTraceForObjects _returnvalue (Math|Vector|MakeVector 0.0 (/ (Variables|Default|Getspeed) 1e+02) 0.0) (Utilities|Array|MakeArray "ObjectTypeQuery5") false 0 "None"))
      (if _returnvalue_6 ; Obstacle?
        (bind _returnvalue_7 (Class|KismetSystemLibrary|BoxOverlapActorsNEW (+ _returnvalue "0,-350.000000, 0" (Math|Vector|MakeVector (/ (* (Variables|Default|Getspeed) 3e+02) 2.0) 0.0 0.0)) (Math|Vector|MakeVector (* (Variables|Default|Getspeed) 3e+02) 3.5e+02 0.0) (Utilities|Array|MakeArray "ObjectTypeQuery5"))) ; Left Box clear?
        (if _returnvalue_7
          (bind _asbot_car (Utilities|Casting|CastToBotCar (.HitActor (Collision|BreakHitResult _outhit))))
          (if (< (Variables|BotCar_C|Getspeed _asbot_car) (Variables|Default|Getspeed))
            (Variables|Default|Setspeed (Variables|BotCar_C|Getspeed _asbot_car)))
          (else
            (Variables|Default|Setstate "NewEnumerator1")
            (Variables|Default|SetendPosition (+ _y_3 -3.5e+02))
            (Variables|Default|SetchangePosition (+ _y_3 -175.0))))
        (else
          (Variables|Default|Setspeed (Variables|Default|GetmaxSpeed))
          (bind _returnvalue_8 (Class|KismetSystemLibrary|BoxOverlapActorsNEW (+ _returnvalue "0,350.000000, 0" (Math|Vector|MakeVector (/ (* (Variables|Default|Getspeed) 3e+02) 2.0) 0.0 0.0)) (Math|Vector|MakeVector (* (Variables|Default|Getspeed) 3e+02) 3.5e+02 0.0) (Utilities|Array|MakeArray "ObjectTypeQuery5"))) ; Right Box clear?
          (if (not _returnvalue_8)
            (Variables|Default|Setstate "NewEnumerator2")
            (Variables|Default|SetendPosition (+ _y_3 3.5e+02))
            (Variables|Default|SetchangePosition (+ _y_3 175.0))))))
    (:NewEnumerator1
      ;[1 1 1] Drive Left
      (if (>= (Variables|Default|GetendPosition) _y_2)
        (Variables|Default|Setstate "NewEnumerator0")
        (Development|PrintString "Drive")
        (else
          (if (>= (Variables|Default|GetchangePosition) _y_2)
            (Variables|Default|Setdirection 0.1)
            (else
              (Variables|Default|Setdirection -0.1)))
          (CallFunction|Rotate (Variables|Default|Getdirection)))))
    (:NewEnumerator2
      ;[1 1 1] Drive Right
      (if (>= _y (Variables|Default|GetendPosition))
        (Variables|Default|Setstate "NewEnumerator0")
        (Development|PrintString "Drive")
        (else
          (if (>= _y (Variables|Default|GetchangePosition))
            (Variables|Default|Setdirection -0.1)
            (else
              (Variables|Default|Setdirection 0.1)))
          (CallFunction|Rotate (Variables|Default|Getdirection)))))))

(event EventBeginPlay
  ;[1 1 1] Init
  (Variables|Default|Setstate "NewEnumerator0")
  (bind _output_get (Variables|Default|SetmaxSpeed (Math|Random|RandomFloatinRange 1e+03 3e+03)))
  (Variables|Default|Setspeed _output_get))

(fn ConstructionScript)

(fn IsonGround
  (bind _returnvalue (Transformation|GetActorLocation))
  (bind _outhit (Collision|LineTraceByChannel _returnvalue (+ _returnvalue "0, 0,-200.000000") "TraceTypeQuery1" false 0 "None"))
  (return (< (Math|Vector|VectorLength (- (Transformation|GetActorLocation) (.Location (Collision|BreakHitResult _outhit)))) 8e+01)))

(fn Rotate
  (params (direction :type Float%20%28single-precision%29))
  (bind _returnvalue (Transformation|GetActorRightVector))
  (bind _nearground (CallFunction|IsonGround))
  (if _nearground
    ;[1 1 1] car rotation
    (Class|PrimitiveComponent|AddForceatLocation (* (* _returnvalue direction) -1.7e+06) (+ (* _returnvalue -2e+02) (Transformation|GetActorLocation) (* (Transformation|GetActorForwardVector) -2e+02)) "None")
    ;[1 1 1] (OLD) instant yaw rotation
    (Transformation|SetActorRotation (Class|KismetMathLibrary|MakeRot 0.0 (+ (.Yaw (Class|KismetMathLibrary|BreakRot (Transformation|GetActorRotation))) (* direction 2.0)) 0.0))))